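; PC_Corvus is the Corvus player character Blueprint, extending its parent's init, state reset and parry logic.
; Init starts the Corvus AnimBP, attaches the dynamic camera target to the mesh's camera socket, and spawns an avoid-agent proxy.
; That proxy teleports to the character when activated for dodge detection and can be deactivated.
; A failed parry becomes a Bounce when the equipped saber has its parry-not-fail skill flag.
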(event EventInit
  (|CallParentFunction)
  ;[1 1 1] AnimBP Init
  (bind _asanim_bp_corvus (Utilities|Casting|CastToAnimBP_Corvus (Components|SkeletalMesh|GetAnimInstance (Variables|Character|GetMesh))))
  (Default|Init _asanim_bp_corvus)
  ;[1 1 1] 動態攝影機Attach To Bone
  (Transformation|AttachComponentToComponent (Variables|Default|GetDynamicCameraTarget) (Variables|Character|GetMesh) "camera" "SnapToTarget" "SnapToTarget" "KeepRelative" true)
  ;[1 1 1] 生成迴避判定代理者
  (bind _returnvalue (Game|SpawnActorfromClass "/Game/GameAsset/BP/Character/Player/PCA_AvoidAgent.PCA_AvoidAgent_C" (Math|Transform|MakeTransform "0, 0, 0" "0, 0, 0" "1,1,1") "Undefined" self 0))
  (Default|Init _returnvalue self)
  (Variables|AvoidAgent|Setref_AvoidAgent _returnvalue))

(event EventReState
  (|CallParentFunction)
  (CallFunction|StopMontage "NewEnumerator0" 0.0))

(fn ConstructionScript
  (|CallParentFunction))

(fn ParryTest
  (params (Attacker :type Game%20Character%20Base%20Object%20Reference) (AttackData :type F%20Attack%20Action%20Data%20Structure))
  (bind _result (|CallParentFunction Attacker AttackData))
  (switch Utilities|FlowControl|Switch|SwitchonEParryResult _result
    (:NewEnumerator0
      _)
    (:NewEnumerator3
      _)
    (:NewEnumerator1
      _)
    (:NewEnumerator2
      (bind _asweapon_saber (Utilities|Casting|CastToWeapon_Saber (Variables|/Game/GameAsset/BP/Character/WeaponSystem/WeaponSystem.WeaponSystem_C|GetCurrentWeapon (Variables|Default|GetWeaponSystem)))
        (:then
          (if (Variables|/Game/GameAsset/BP/Character/Player/Corvus/Weapon/Weapon_Saber.Weapon_Saber_C|GetSkillFlag_ParryNotFail _asweapon_saber)
            (return "NewEnumerator1")
            (else
              _)))
        (:CastFailed
          _))))
  (return _result))

(fn ActiveAvoidAgent
  (bind _ref_avoidagent (Variables|AvoidAgent|Getref_AvoidAgent))
  (Transformation|SetActorLocation _ref_avoidagent (Transformation|GetActorLocation) false true)
  (Default|Active _ref_avoidagent))

(fn UnactiveAvoidAgent
  (Default|Unactive (Variables|AvoidAgent|Getref_AvoidAgent)))