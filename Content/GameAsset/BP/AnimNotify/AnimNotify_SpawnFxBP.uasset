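; Animation notify that spawns an effect Blueprint actor on the animated mesh when the notify fires.
; If the FxBP class is valid, it spawns the actor at the AttackSocket's location and rotation with the configured Scale, then attaches it to that socket.
; Attachment snaps location and rotation while keeping relative scale.
; Spawning is skipped when the spot is colliding, and the attach has no validity check on the spawned actor.
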(fn ReceivedNotify
  (params (MeshComp :type Skeletal%20Mesh%20Component%20Object%20Reference) (Animation :type Anim%20Sequence%20Base%20Object%20Reference))
  (bind _fxbp (Variables|Default|GetFxBP))
  (bind _attacksocket (Variables|Default|GetAttackSocket))
  (if (Utilities|IsValidClass _fxbp)
    (bind _returnvalue (Game|SpawnActorfromClass _fxbp (Math|Transform|MakeTransform (Transformation|GetSocketLocation MeshComp _attacksocket) (Transformation|GetSocketRotation MeshComp _attacksocket) (Variables|Default|GetScale)) "DontSpawnIfColliding" 0 0))
    (Transformation|AttachComponentToComponent _returnvalue MeshComp (Variables|Default|GetAttackSocket) "SnapToTarget" "SnapToTarget" "KeepRelative" true)
    (return false)))